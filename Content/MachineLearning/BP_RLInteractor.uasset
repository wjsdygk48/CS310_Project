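; Learning Agents interactor that lets an RL policy adjust the AI's difficulty scale based on how competitive combat is.
; Observes the current difficulty scale and half the player-minus-AI difference in summed team HP and living units from BP_CombatSystem.
; Applies a single float action to each BP_AiAgent through SetDifficultyScale.
; Separate HP, unit and reward-direction observations are left unwired.
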(event EventSetupObservations
  (bind _returnvalue (Class|FloatObservation|AddFloatObservation 0 "CompScore" 1.0))
  (Variables|Observations|SetCompScoreObs _returnvalue)
  (bind _returnvalue_2 (Class|FloatObservation|AddFloatObservation 0 "DiffScale" 1.0))
  (Variables|Observations|SetDiffScaleObs _returnvalue_2))

(event EventSetObservations
  (params (AgentIds :type Array%20of%20Integers))
  (CallFunction|CalculateHp)
  (CallFunction|CalculateUnits)
  (bind _competitivescore (CallFunction|CalculateCompetitiveScore))
  (Variables|ObsValues|SetCompScore (/ _competitivescore 2.0))
  (Variables|ObsValues|SetDiffScale (Variables|/Game/Core/Units/AI/BP_AiAgent.BP_AiAgent_C|GetDifficultyScale (Variables|Default|GetAiAgent)))
  (for _array_element AgentIds
    (Class|FloatObservation|SetFloatObservation (Variables|Observations|GetCompScoreObs) _array_element (Variables|ObsValues|GetCompScore))
    (Class|FloatObservation|SetFloatObservation (Variables|Observations|GetDiffScaleObs) _array_element (Variables|ObsValues|GetDiffScale))
    (Development|PrintString (Utilities|String|Append "Competitive Score: " (Utilities|String|ToString(Float) (Variables|ObsValues|GetCompScore)) ", Difficulty Scale Value: " (Utilities|String|ToString(Float) (Variables|ObsValues|GetDiffScale))))))

(event EventSetupActions
  (bind _returnvalue (Class|FloatAction|AddFloatAction 0 "DiffScaleAction" 1.0))
  (Variables|Default|SetDiffScaleAction _returnvalue))

(event EventBeginPlay
  (bind _returnvalue (Actor|GetActorOfClass "/Game/Core/Combat/BP_CombatSystem.BP_CombatSystem_C"))
  (Variables|Default|SetCombatSystem _returnvalue)
  (bind _returnvalue_2 (Actor|GetActorOfClass "/Game/Core/Units/AI/BP_AiAgent.BP_AiAgent_C"))
  (Variables|Default|SetAiAgent _returnvalue_2))

(event EventGetActions
  (params (AgentIds :type Array%20of%20Integers))
  (for _array_element AgentIds
    (bind _returnvalue (Class|FloatAction|GetFloatAction (Variables|Default|GetDiffScaleAction) _array_element))
    (Default|SetDifficultyScale (Class|LearningAgentsManagerComponent|GetAgent _array_element "/Game/Core/Units/AI/BP_AiAgent.BP_AiAgent_C") _returnvalue)))

(fn IsAgentAlive
  (params (AgentId :type Integer))
  (if (<= (Utilities|Struct|BreakS_UnitData_Stats (Utilities|Struct|BreakS_UnitData (Variables|/Game/Core/Units/BP_Unit.BP_Unit_C|GetUnitData (Variables|/Game/Core/Units/AI/BP_UnitAi.BP_UnitAi_C|GetUnit (Class|LearningAgentsManagerComponent|GetAgent AgentId "/Game/Core/Units/AI/BP_UnitAi.BP_UnitAi_C"))))) 0)
    (return false)
    (else
      (return true))))

(fn NormaliseFloatObs
  (params (FloatObs :type Float%20%28double-precision%29))
  (return (- (* FloatObs 2.0) 1.0)))

(fn SetHpObs
  (params (AgentID :type Integer))
  (bind _combatsystem (Variables|Default|GetCombatSystem))
  (Variables|ObsValues|SetAiCurrentHp 0.0)
  (Variables|ObsValues|SetPlayerCurrentHp 0.0)
  (bind _currenttotalhp (Default|GetCurrentTotalTeamHp _combatsystem 1))
  (Variables|ObsValues|SetAiCurrentHp (CallFunction|NormaliseFloatObs _currenttotalhp))
  (bind _currenttotalhp_2 (Default|GetCurrentTotalTeamHp _combatsystem))
  (Variables|ObsValues|SetPlayerCurrentHp (CallFunction|NormaliseFloatObs _currenttotalhp_2))
  (Class|FloatObservation|SetFloatObservation (Variables|Observations|GetAiHpObs) AgentID (Variables|ObsValues|GetAiCurrentHp))
  (Class|FloatObservation|SetFloatObservation (Variables|Observations|GetPlayerHpObs) AgentID (Variables|ObsValues|GetPlayerCurrentHp)))

(fn SetUnitsObs
  (params (AgentId :type Integer))
  (bind _combatsystem (Variables|Default|GetCombatSystem))
  (Variables|ObsValues|SetAiLivingUnits 0.0)
  (Variables|ObsValues|SetPlayerLivingUnits 0.0)
  (bind _livingunits (Default|GetLivingUnitCount _combatsystem 1))
  (Variables|ObsValues|SetAiLivingUnits (CallFunction|NormaliseFloatObs _livingunits))
  (bind _livingunits_2 (Default|GetLivingUnitCount _combatsystem))
  (Variables|ObsValues|SetPlayerLivingUnits (CallFunction|NormaliseFloatObs _livingunits_2))
  (Class|FloatObservation|SetFloatObservation (Variables|Observations|GetAiLivingUnitsObs) AgentId (Variables|ObsValues|GetAiLivingUnits))
  (Class|FloatObservation|SetFloatObservation (Variables|Observations|GetPlayerLivingUnitsObs) AgentId (Variables|ObsValues|GetPlayerLivingUnits)))

(fn CalculateCompetitiveScore
  ;[1 1 1] Calculate the score to gauge how competitive the game was (player wins => positive reward, ai wins => negative reward)
  (return (- (+ (Variables|ObsValues|GetPlayerCurrentHp) (Variables|ObsValues|GetPlayerLivingUnits)) (+ (Variables|ObsValues|GetAiCurrentHp) (Variables|ObsValues|GetAiLivingUnits)))))

(fn CalculateHp
  (bind _combatsystem (Variables|Default|GetCombatSystem))
  (Variables|ObsValues|SetAiCurrentHp 0.0)
  (Variables|ObsValues|SetPlayerCurrentHp 0.0)
  (bind _currenttotalhp (Default|GetCurrentTotalTeamHp _combatsystem 1))
  (Variables|ObsValues|SetAiCurrentHp _currenttotalhp)
  (bind _currenttotalhp_2 (Default|GetCurrentTotalTeamHp _combatsystem))
  (Variables|ObsValues|SetPlayerCurrentHp _currenttotalhp_2))

(fn CalculateUnits
  (bind _combatsystem (Variables|Default|GetCombatSystem))
  (Variables|ObsValues|SetAiLivingUnits 0.0)
  (Variables|ObsValues|SetPlayerLivingUnits 0.0)
  (bind _livingunits (Default|GetLivingUnitCount _combatsystem 1))
  (Variables|ObsValues|SetAiLivingUnits _livingunits)
  (bind _livingunits_2 (Default|GetLivingUnitCount _combatsystem))
  (Variables|ObsValues|SetPlayerLivingUnits _livingunits_2))