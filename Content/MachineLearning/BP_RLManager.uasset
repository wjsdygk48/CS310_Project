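; Manager actor that drives Learning Agents reinforcement learning for the turn-based combat system.
; BeginPlay sets up the interactor, policy (on DA_RLNetwork) and trainer, then binds to combat system events.
; Training steps run on unit turn start and end rather than on Tick, with a final step before training ends as combat finishes.
; The construction script finds the combat system and player actions actors by class.
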(event Custom|Event_UnitTurnStarted
  (params (Unit :type BP%20Unit%20Object%20Reference))
  (Class|LearningAgentsTrainer|RunTraining (Variables|Default|GetBP_Trainer) (Variables|Trainer|GetTrainer%20Training%20Settings) (Variables|Trainer|GetTrainer%20Game%20Settings) (Variables|Trainer|GetTrainer%20Path%20Settings) (Variables|Trainer|GetCritic%20Settings) false true true))

(event Custom|Event_CombatFinishing
  (params (WinningTeamIndex :type Integer))
  (Class|LearningAgentsTrainer|RunTraining (Variables|Default|GetBP_Trainer) (Variables|Trainer|GetTrainer%20Training%20Settings) (Variables|Trainer|GetTrainer%20Game%20Settings) (Variables|Trainer|GetTrainer%20Path%20Settings) (Variables|Trainer|GetCritic%20Settings) false true true)
  (Class|LearningAgentsTrainer|EndTraining (Variables|Default|GetBP_Trainer))
  (Development|PrintString "Ending Training"))

(event Custom|Event_UnitTurnEnded
  (params (Unit :type BP%20Unit%20Object%20Reference))
  (Class|LearningAgentsTrainer|RunTraining (Variables|Default|GetBP_Trainer) (Variables|Trainer|GetTrainer%20Training%20Settings) (Variables|Trainer|GetTrainer%20Game%20Settings) (Variables|Trainer|GetTrainer%20Path%20Settings) (Variables|Trainer|GetCritic%20Settings) false true true))

(event EventTick
  (params (DeltaSeconds :type Float%20%28single-precision%29)))

(event EventBeginPlay
  (Utilities|FlowControl|Sequence
    (:then_0
      (Class|LearningAgentsInteractor|SetupInteractor (Variables|Default|GetBP_Interactor)))
    (:then_1
      (Class|LearningAgentsPolicy|SetupPolicy (Variables|Default|GetBP_Policy) (Variables|Default|GetBP_Interactor) (Variables|Default|GetPolicy%20Settings) "/Game/MachineLearning/DA_RLNetwork.DA_RLNetwork"))
    (:then_2
      (Class|LearningAgentsTrainer|SetupTrainer (Variables|Default|GetBP_Trainer) (Variables|Default|GetBP_Interactor) (Variables|Default|GetBP_Policy) 0 (Variables|Trainer|GetTrainer%20Settings)))
    (:then_3
      (EventDispatchers|BindEventtoOnUnitTurnStarted (Variables|Default|GetCombatSystem) (delegate Custom|Event_UnitTurnStarted))
      (EventDispatchers|BindEventtoOnUnitTurnEnded (Variables|Default|GetCombatSystem) (delegate Custom|Event_UnitTurnEnded))
      (EventDispatchers|BindEventtoOnCombatFinishing (Variables|Default|GetCombatSystem) (delegate Custom|Event_CombatFinishing)))))

(fn ConstructionScript
  (bind _returnvalue (Actor|GetActorOfClass "/Game/Core/Combat/BP_CombatSystem.BP_CombatSystem_C"))
  (Variables|Default|SetCombatSystem _returnvalue)
  (bind _returnvalue_2 (Actor|GetActorOfClass "/Game/Core/Player/BP_PlayerActions.BP_PlayerActions_C"))
  (Variables|Default|SetPlayerActions _returnvalue_2))

(fn UnitTurnEnded
  (params (Unit :type BP%20Unit%20Object%20Reference)))