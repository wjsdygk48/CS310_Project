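; Learning Agents trainer that teaches an AI to adapt turn-based combat difficulty, rewarding it when the player leads in team HP and penalizing it when the AI leads.
; Rewards compare both teams' HP each step, with larger ones on every fourth team turn.
; At combat end, rewards scale with consecutive wins and HP gap, weighted by RewardDirection so upsets count double.
; A single GameEnded completion terminates episodes when CombatSystem finishes combat.
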(event EventSetupRewards
  (bind _returnvalue (Class|FloatReward|AddFloatReward 0 "Reward" 1.0))
  (Variables|Default|SetReward _returnvalue))

(event EventSetRewards
  (params (AgentIds :type Array%20of%20Integers))
  (bind _combatsystem (Variables|Default|GetCombatSystem))
  (bind _currenttotalhp (Default|GetCurrentTotalTeamHp _combatsystem 1))
  (Variables|Default|SetAiCurrentHp _currenttotalhp)
  (bind _currenttotalhp_2 (Default|GetCurrentTotalTeamHp _combatsystem))
  (Variables|Default|SetPlayerCurrentHp _currenttotalhp_2)
  (for _array_element AgentIds
    (if (Variables|/Game/Core/Combat/BP_CombatSystem.BP_CombatSystem_C|GetIsFinishingCombat (Variables|Default|GetCombatSystem))
      (CallFunction|FinishGameReward _array_element)
      (else
        (CallFunction|TeamTurnsElapsedReward _array_element)))))

(event EventSetupCompletions
  (bind _returnvalue (Class|ConditionalCompletion|AddConditionalCompletion 0 "GameEnded" "Termination"))
  (Variables|Default|SetGameEndedCompletion _returnvalue))

(event EventSetCompletions
  (params (AgentIds :type Array%20of%20Integers))
  ;[1 1 1] When game has ended terminate and end training
  (for _array_element AgentIds
    (Class|ConditionalCompletion|SetConditionalCompletion (Variables|Default|GetGameEndedCompletion) _array_element (Variables|/Game/Core/Combat/BP_CombatSystem.BP_CombatSystem_C|GetIsFinishingCombat (Variables|Default|GetCombatSystem)))))

(event EventBeginPlay
  (bind _returnvalue (Actor|GetActorOfClass "/Game/Core/Combat/BP_CombatSystem.BP_CombatSystem_C"))
  (Variables|Default|SetCombatSystem _returnvalue)
  (bind _returnvalue_2 (Actor|GetActorOfClass "/Game/Core/Player/BP_PlayerActions.BP_PlayerActions_C"))
  (Variables|Default|SetPlayerActions _returnvalue_2))

(fn FinishGameReward
  (params (AgentId :type Integer))
  (bind _combatsystem (Variables|Default|GetCombatSystem))
  (bind _combatsystem_2 (Variables|Default|GetCombatSystem))
  (bind _teamwinsdata (Variables|/Game/Core/Combat/BP_CombatSystem.BP_CombatSystem_C|GetTeamWinsData _combatsystem))
  (bind _teamwinsdata_2 (Variables|/Game/Core/Combat/BP_CombatSystem.BP_CombatSystem_C|GetTeamWinsData _combatsystem_2))
  ;[1 1 1] Depending on the reward direction give different levels of positive or negative rewards
  (switch Utilities|FlowControl|Switch|SwitchonE_RewardDirection (Variables|Default|GetRewardDirection)
    (:NewEnumerator0
      ;[1 1 1] If the advantaged team wins it is expected and so the rewards are normal, however if the disadvantaged team wins it is unexpected so an extreme reward is given
      (if (== (.winningteamindex _teamwinsdata_2) 1)
        (Class|FloatReward|SetFloatReward (Variables|Default|GetReward) AgentId (+ (* (.consecutivewins _teamwinsdata_2) -5e+01) (- (Variables|Default|GetPlayerCurrentHp) (Variables|Default|GetAiCurrentHp))))
        (Development|PrintString "Ai too hard: lowering difficulty")
        (else
          (Class|FloatReward|SetFloatReward (Variables|Default|GetReward) AgentId (+ (* (.consecutivewins _teamwinsdata_2) 1e+02) (- (Variables|Default|GetPlayerCurrentHp) (Variables|Default|GetAiCurrentHp))))
          (Development|PrintString "Ai too easy: raising difficulty"))))
    (:NewEnumerator1
      (if (== (.winningteamindex _teamwinsdata) 0)
        (Class|FloatReward|SetFloatReward (Variables|Default|GetReward) AgentId (+ (* (.consecutivewins _teamwinsdata) 5e+01) (- (Variables|Default|GetPlayerCurrentHp) (Variables|Default|GetAiCurrentHp))))
        (Development|PrintString "Player is better: raising difficulty")
        (else
          (Class|FloatReward|SetFloatReward (Variables|Default|GetReward) AgentId (+ (* (.consecutivewins _teamwinsdata) -1e+02) (- (Variables|Default|GetPlayerCurrentHp) (Variables|Default|GetAiCurrentHp))))
          (Development|PrintString "Player struggling: lowering difficulty"))))))

(fn TeamTurnsElapsedReward
  (params (AgentId :type Integer))
  (if (and (== (Math|Integer|%(Integer) (Variables|/Game/Core/Combat/BP_CombatSystem.BP_CombatSystem_C|GetTeamTurnNumber (Variables|Default|GetCombatSystem)) 4) 0) (!= (Variables|/Game/Core/Combat/BP_CombatSystem.BP_CombatSystem_C|GetTeamTurnNumber (Variables|Default|GetCombatSystem)) 0))
    (Development|PrintString "TWO TURNS ELAPSED REWARDS: ")
    (if (< (Variables|Default|GetAiCurrentHp) (Variables|Default|GetPlayerCurrentHp))
      (Class|FloatReward|SetFloatReward (Variables|Default|GetReward) AgentId 25.0)
      (Development|PrintString "AI < PLAYER")
      (elif (== (Variables|Default|GetAiCurrentHp) (Variables|Default|GetPlayerCurrentHp))
        (Class|FloatReward|SetFloatReward (Variables|Default|GetReward) AgentId 0.0)
        (Development|PrintString "AI = PLAYER")
        (elif (> (Variables|Default|GetAiCurrentHp) (Variables|Default|GetPlayerCurrentHp))
          (Class|FloatReward|SetFloatReward (Variables|Default|GetReward) AgentId -25.0)
          (Development|PrintString "AI > PLAYER"))))
    (else
      (CallFunction|NormalReward AgentId))))

(fn NormalReward
  (params (AgentId :type Integer))
  (if (< (Variables|Default|GetAiCurrentHp) (Variables|Default|GetPlayerCurrentHp))
    (Class|FloatReward|SetFloatReward (Variables|Default|GetReward) AgentId 1e+01)
    (elif (== (Variables|Default|GetAiCurrentHp) (Variables|Default|GetPlayerCurrentHp))
      (Class|FloatReward|SetFloatReward (Variables|Default|GetReward) AgentId 0.0)
      (elif (> (Variables|Default|GetAiCurrentHp) (Variables|Default|GetPlayerCurrentHp))
        (Class|FloatReward|SetFloatReward (Variables|Default|GetReward) AgentId -1e+01)))))