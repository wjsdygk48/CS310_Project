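; Player input hub for grid-based tactical combat that tracks the hovered and selected tile and unit, and spawns the default units.
; Left and right clicks run swappable spawned action actors, which repeat on hover changes while the button is held.
; Selection highlights movement tiles by unit type, limiting moves to unoccupied ones.
; Combat system events manage the combat widget and turn selection, while spell choice switches left click between moving and casting.
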(event Custom|OnHoveredTileChanged
  (bind _selectedaction_leftclick (Variables|Actions|GetSelectedAction_LeftClick))
  (bind _selectedaction_rightclick (Variables|Actions|GetSelectedAction_RightClick))
  (Utilities|FlowControl|Sequence
    (:then_0
      (Utilities|IsValid _selectedaction_leftclick
        (:Is%20Valid
          (Default|ExecuteHoveredAction _selectedaction_leftclick (Variables|References|GetHoveredTile))
          (if (Variables|Actions|GetIsLeftClickDown)
            (Default|ExecuteAction (Variables|Actions|GetSelectedAction_LeftClick) (Variables|References|GetHoveredTile))))))
    (:then_1
      (Utilities|IsValid _selectedaction_rightclick
        (:Is%20Valid
          (Default|ExecuteHoveredAction _selectedaction_rightclick (Variables|References|GetHoveredTile))
          (if (Variables|Actions|GetIsRightClickDown)
            (Default|ExecuteAction (Variables|Actions|GetSelectedAction_RightClick) (Variables|References|GetHoveredTile))))))))

(event EventBeginPlay
  (bind _returnvalue (Actor|GetActorOfClass "/Game/Core/Grid/BP_Grid.BP_Grid_C"))
  (Variables|Components|SetGrid _returnvalue)
  (bind _returnvalue_2 (Actor|GetActorOfClass "/Game/Core/Combat/BP_CombatSystem.BP_CombatSystem_C"))
  (Variables|Components|SetCombatSystem _returnvalue_2)
  (CallFunction|CreateDefaultUnits)
  (EventDispatchers|BindEventtoOnCombatStarted (Variables|Components|GetCombatSystem) (EventDispatchers|CreateEvent :!event OnCombatStarted))
  (EventDispatchers|BindEventtoOnCombatEnded (Variables|Components|GetCombatSystem) (EventDispatchers|CreateEvent :!event OnCombatEnded))
  (EventDispatchers|BindEventtoOnUnitTurnStarted (Variables|Components|GetCombatSystem) (EventDispatchers|CreateEvent :!event OnUnitTurnStarted))
  (EventDispatchers|BindEventtoOnUnitTurnEnded (Variables|Components|GetCombatSystem) (EventDispatchers|CreateEvent :!event OnUnitTurnEnded))
  (Input|EnableInput (Game|GetPlayerController 0)))

(event EventTick
  (params (DeltaSeconds :type Float%20%28single-precision%29))
  (Actions|UpdateHoveredTileandUnit))

(event Input|MouseEvents|LeftMouseButton
  (params (Key :type Key%20Structure :default "None"))
  (:Pressed
    (Actions|UpdateHoveredTileandUnit)
    (Variables|Actions|SetIsLeftClickDown true)
    (Utilities|IsValid (Variables|Actions|GetSelectedAction_LeftClick)
      (:Is%20Valid
        (Default|ExecuteAction (Variables|Actions|GetSelectedAction_LeftClick) (Variables|References|GetHoveredTile)))))
  (:Released
    (Variables|Actions|SetIsLeftClickDown false)))

(event Input|MouseEvents|RightMouseButton
  (params (Key :type Key%20Structure :default "None"))
  (:Pressed
    (Actions|UpdateHoveredTileandUnit)
    (Variables|Actions|SetIsRightClickDown true)
    (Utilities|IsValid (Variables|Actions|GetSelectedAction_RightClick)
      (:Is%20Valid
        (Default|ExecuteAction (Variables|Actions|GetSelectedAction_RightClick) (Variables|References|GetHoveredTile)))))
  (:Released
    (Variables|Actions|SetIsRightClickDown false)))

(fn ConstructionScript)

(fn UpdateHoveredTileandUnit
  (Utilities|FlowControl|Sequence
    (:then_0
      (bind _unit (Actions|GetUnitUnderCursor))
      (if (!= _unit (Variables|References|GetHoveredUnit))
        (Utilities|FlowControl|Sequence
          (:then_0
            (Utilities|IsValid (Variables|References|GetHoveredUnit)
              (:Is%20Valid
                (Default|SetIsHovered (Variables|References|GetHoveredUnit) false))))
          (:then_1
            (bind _output_get (Variables|References|SetHoveredUnit _unit))
            (Utilities|IsValid _output_get
              (:Is%20Valid
                (Default|SetIsHovered _output_get true)))))))
    (:then_1
      (Utilities|IsValid (Variables|References|GetHoveredUnit) ; If the index is valid use the unit index
        (:Is%20Valid
          (LocalVariables|SetNewIndex (Variables|/Game/Core/Units/BP_Unit.BP_Unit_C|GetIndex (Variables|References|GetHoveredUnit))))
        (:Is%20Not%20Valid
          (bind _index (Default|GetTileIndexUnderCursor (Variables|Components|GetGrid))) ; If not use the index of the tile below it
          (LocalVariables|SetNewIndex _index)))
      (if (!= (LocalVariables|GetNewIndex) (Variables|References|GetHoveredTile))
        (Default|RemoveStatefromTile (Variables|Components|GetGrid) (Variables|References|GetHoveredTile) "NewEnumerator1")
        (Variables|References|SetHoveredTile (LocalVariables|GetNewIndex))
        (Default|AddStatetoTile (Variables|Components|GetGrid) (Variables|References|GetHoveredTile) "NewEnumerator1")
        (CallFunction|OnHoveredTileChanged)))))

(fn SetSelectedActions
  (params (LeftAction :type BP%20Action%20Class%20Reference) (RightAction :type BP%20Action%20Class%20Reference))
  (Utilities|FlowControl|Sequence
    (:then_0
      (Utilities|IsValid (Variables|Actions|GetSelectedAction_LeftClick)
        (:Is%20Valid
          (Actor|DestroyActor (Variables|Actions|GetSelectedAction_LeftClick))
          (Variables|Actions|SetSelectedAction_LeftClick 0))
        (:Is%20Not%20Valid
          _))
      (if (Utilities|IsValidClass LeftAction)
        (bind _returnvalue (Game|SpawnActorfromClass LeftAction (Math|Transform|MakeTransform "0, 0, 0" "0, 0, 0" "1.000000,1.000000,1.000000") "AlwaysSpawn" "MultiplyWithRoot" 0 self 0))
        (Variables|Actions|SetSelectedAction_LeftClick _returnvalue)))
    (:then_1
      (Utilities|IsValid (Variables|Actions|GetSelectedAction_RightClick)
        (:Is%20Valid
          (Actor|DestroyActor (Variables|Actions|GetSelectedAction_RightClick))
          (Variables|Actions|SetSelectedAction_RightClick 0))
        (:Is%20Not%20Valid
          _))
      (if (Utilities|IsValidClass RightAction)
        (bind _returnvalue_2 (Game|SpawnActorfromClass RightAction (Math|Transform|MakeTransform "0, 0, 0" "0, 0, 0" "1.000000,1.000000,1.000000") "AlwaysSpawn" "MultiplyWithRoot" 0 self 0))
        (Variables|Actions|SetSelectedAction_RightClick _returnvalue_2)))
    (:then_2
      (Default|CallOnSelectedActionsChanged (Variables|Actions|GetSelectedAction_LeftClick) (Variables|Actions|GetSelectedAction_RightClick)))))

(fn GetUnitUnderCursor
  (params (PlayerIndex :type Integer))
  (bind _returnvalue (Game|GetPlayerController PlayerIndex))
  (bind (_hitresult _returnvalue_2) (Game|Player|GetHitResultUnderCursorbyChannel _returnvalue "TraceTypeQuery4" false))
  (if _returnvalue_2 ; Mouse ove r unit then return unit else get unit on tile
    (return (.AsBP%20Unit (Utilities|Casting|CastToBP_Unit (.HitActor (Collision|BreakHitResult _hitresult)))))
    (else
      (bind _index (Default|GetTileIndexUnderCursor (Variables|Components|GetGrid) PlayerIndex)) ; Get the index of the tile and find the matching tile data with the unit on tile
      (return (.UnitOnTile (Utilities|Struct|BreakS_TileData (.Value (Utilities|Map|Find (Variables|/Game/Core/Grid/BP_Grid.BP_Grid_C|GetGridTiles (Variables|Components|GetGrid)) _index))))))))

(fn SetSelectedTileandUnit
  (params (Index :type Int%20Point%20Structure))
  (UnitReachableTiles|ResetReachableTiles) ; Reset movement tiles for previous unit to default
  (Utilities|Array|Clear (Variables|UnitReachableTiles|GetReachableIndexes)) ; Clear the array
  (Utilities|FlowControl|Sequence
    (:then_0
      (if (!= (Variables|References|GetSelectedTile) Index) ; If the selected tiles are different
        (Default|RemoveStatefromTile (Variables|Components|GetGrid) (Variables|References|GetSelectedTile) "NewEnumerator2") ; Remove the state from the previous tile
        (bind _output_get (Variables|References|SetSelectedTile Index)) ; Set new tile
        (Development|PrintString (Utilities|String|ToString(Integer) _output_get))
        (Default|AddStatetoTile (Variables|Components|GetGrid) (Variables|References|GetSelectedTile) "NewEnumerator2") ; Add state to the new tile
        (else
          (Default|RemoveStatefromTile (Variables|Components|GetGrid) (Variables|References|GetSelectedTile) "NewEnumerator2") ; Remove the state from the previous tile
          (Variables|References|SetSelectedTile (Utilities|Struct|MakeIntPoint -999 -999)) ; Set invalid tile
        ))
      (Default|CallOnSelectedTileChanged (Variables|References|GetSelectedTile)))
    (:then_1
      (LocalVariables|SetNewUnit (.UnitOnTile (Utilities|Struct|BreakS_TileData (.Value (Utilities|Map|Find (Variables|/Game/Core/Grid/BP_Grid.BP_Grid_C|GetGridTiles (Variables|Components|GetGrid)) (Variables|References|GetSelectedTile))))))
      (if (!= (Variables|References|GetSelectedUnit) (LocalVariables|GetNewUnit))
        (Utilities|FlowControl|Sequence
          (:then_0
            (Utilities|IsValid (Variables|References|GetSelectedUnit)
              (:Is%20Valid
                (Default|SetIsSelected (Variables|References|GetSelectedUnit) false))))
          (:then_1
            (bind _output_get_2 (Variables|References|SetSelectedUnit (LocalVariables|GetNewUnit)))
            (Utilities|IsValid _output_get_2
              (:Is%20Valid
                (Default|SetIsSelected _output_get_2 true)
                (UnitReachableTiles|GetUnitReachableRange _output_get_2)
                (UnitReachableTiles|SetReachableTiles)))))))))

(fn GetUnitReachableRange
  (params (SelectedUnit :type BP%20Unit%20Object%20Reference))
  (Variables|UnitReachableTiles|SetCurrentUnitIndex (Variables|/Game/Core/Units/BP_Unit.BP_Unit_C|GetIndex SelectedUnit))
  (switch Utilities|FlowControl|Switch|SwitchonE_UnitType (Variables|/Game/Core/Units/BP_Unit.BP_Unit_C|GetUnitType SelectedUnit) ; Depending on the unit type call different functions
    (:NewEnumerator0
      (UnitReachableTiles|GetSwordsmanReachable))
    (:NewEnumerator1
      (UnitReachableTiles|GetRangerReachable))
    (:NewEnumerator2
      (UnitReachableTiles|GetMageReachable)))
  (return))

(fn GetSwordsmanReachable
  (bind _currentunitindex (Variables|UnitReachableTiles|GetCurrentUnitIndex))
  (bind _currentunitindex_2 (Variables|UnitReachableTiles|GetCurrentUnitIndex))
  (bind _currentunitindex_3 (Variables|UnitReachableTiles|GetCurrentUnitIndex))
  (bind _currentunitindex_4 (Variables|UnitReachableTiles|GetCurrentUnitIndex))
  (for _index (range 1 2)
    (if (Default|IsIndexValid (Variables|Components|GetGrid) (Utilities|Struct|MakeIntPoint (+ _index (.x _currentunitindex_2)) (.y _currentunitindex_2)))
      (Utilities|Array|AddUnique (Variables|UnitReachableTiles|GetReachableIndexes) (Utilities|Struct|MakeIntPoint (+ _index (.x _currentunitindex_2)) (.y _currentunitindex_2))))
    (if (Default|IsIndexValid (Variables|Components|GetGrid) (Utilities|Struct|MakeIntPoint (- (.x _currentunitindex) _index) (.y _currentunitindex)))
      (Utilities|Array|AddUnique (Variables|UnitReachableTiles|GetReachableIndexes) (Utilities|Struct|MakeIntPoint (- (.x _currentunitindex) _index) (.y _currentunitindex)))))
  (for _index_2 (range 1 2)
    (if (Default|IsIndexValid (Variables|Components|GetGrid) (Utilities|Struct|MakeIntPoint (.x _currentunitindex_3) (+ (.y _currentunitindex_3) _index_2)))
      (Utilities|Array|AddUnique (Variables|UnitReachableTiles|GetReachableIndexes) (Utilities|Struct|MakeIntPoint (.x _currentunitindex_3) (+ (.y _currentunitindex_3) _index_2))))
    (if (Default|IsIndexValid (Variables|Components|GetGrid) (Utilities|Struct|MakeIntPoint (.x _currentunitindex_4) (- (.y _currentunitindex_4) _index_2)))
      (Utilities|Array|AddUnique (Variables|UnitReachableTiles|GetReachableIndexes) (Utilities|Struct|MakeIntPoint (.x _currentunitindex_4) (- (.y _currentunitindex_4) _index_2))))))

(fn GetRangerReachable
  (bind _currentunitindex (Variables|UnitReachableTiles|GetCurrentUnitIndex))
  (bind _currentunitindex_2 (Variables|UnitReachableTiles|GetCurrentUnitIndex))
  (bind _currentunitindex_3 (Variables|UnitReachableTiles|GetCurrentUnitIndex))
  (bind _currentunitindex_4 (Variables|UnitReachableTiles|GetCurrentUnitIndex))
  (bind _returnvalue (+ (.x _currentunitindex_3) 1))
  (bind _returnvalue_2 (+ (.y _currentunitindex_3) 0))
  (bind _returnvalue_3 (+ (.x _currentunitindex_4) -1))
  (bind _returnvalue_4 (+ (.y _currentunitindex_4) 0))
  (bind _returnvalue_5 (+ (.x _currentunitindex) 0))
  (bind _returnvalue_6 (+ (.y _currentunitindex) 1))
  (bind _returnvalue_7 (+ (.x _currentunitindex_2) 0))
  (bind _returnvalue_8 (+ (.y _currentunitindex_2) -1))
  (if (Default|IsIndexValid (Variables|Components|GetGrid) (Utilities|Struct|MakeIntPoint _returnvalue_5 _returnvalue_6))
    (Utilities|Array|AddUnique (Variables|UnitReachableTiles|GetReachableIndexes) (Utilities|Struct|MakeIntPoint _returnvalue_5 _returnvalue_6)))
  (if (Default|IsIndexValid (Variables|Components|GetGrid) (Utilities|Struct|MakeIntPoint _returnvalue_7 _returnvalue_8))
    (Utilities|Array|AddUnique (Variables|UnitReachableTiles|GetReachableIndexes) (Utilities|Struct|MakeIntPoint _returnvalue_7 _returnvalue_8)))
  (if (Default|IsIndexValid (Variables|Components|GetGrid) (Utilities|Struct|MakeIntPoint _returnvalue _returnvalue_2))
    (Utilities|Array|AddUnique (Variables|UnitReachableTiles|GetReachableIndexes) (Utilities|Struct|MakeIntPoint _returnvalue _returnvalue_2)))
  (if (Default|IsIndexValid (Variables|Components|GetGrid) (Utilities|Struct|MakeIntPoint _returnvalue_3 _returnvalue_4))
    (Utilities|Array|AddUnique (Variables|UnitReachableTiles|GetReachableIndexes) (Utilities|Struct|MakeIntPoint _returnvalue_3 _returnvalue_4))))

(fn GetMageReachable
  (bind _currentunitindex (Variables|UnitReachableTiles|GetCurrentUnitIndex))
  (bind _currentunitindex_2 (Variables|UnitReachableTiles|GetCurrentUnitIndex))
  (bind _currentunitindex_3 (Variables|UnitReachableTiles|GetCurrentUnitIndex))
  (bind _currentunitindex_4 (Variables|UnitReachableTiles|GetCurrentUnitIndex))
  (bind _currentunitindex_5 (Variables|UnitReachableTiles|GetCurrentUnitIndex))
  (bind _currentunitindex_6 (Variables|UnitReachableTiles|GetCurrentUnitIndex))
  (bind _currentunitindex_7 (Variables|UnitReachableTiles|GetCurrentUnitIndex))
  (bind _currentunitindex_8 (Variables|UnitReachableTiles|GetCurrentUnitIndex))
  (bind _returnvalue (+ (.y _currentunitindex_8) -1))
  (bind _returnvalue_2 (+ (.x _currentunitindex_8) -1))
  (bind _returnvalue_3 (+ (.x _currentunitindex_5) 1))
  (bind _returnvalue_4 (+ (.y _currentunitindex_5) 0))
  (bind _returnvalue_5 (+ (.x _currentunitindex_2) -1))
  (bind _returnvalue_6 (+ (.y _currentunitindex_2) 1))
  (bind _returnvalue_7 (+ (.x _currentunitindex_6) -1))
  (bind _returnvalue_8 (+ (.y _currentunitindex_6) 0))
  (bind _returnvalue_9 (+ (.x _currentunitindex_3) 0))
  (bind _returnvalue_10 (+ (.y _currentunitindex_3) 1))
  (bind _returnvalue_11 (+ (.x _currentunitindex) 1))
  (bind _returnvalue_12 (+ (.y _currentunitindex) 1))
  (bind _returnvalue_13 (+ (.x _currentunitindex_7) 1))
  (bind _returnvalue_14 (+ (.y _currentunitindex_7) -1))
  (bind _returnvalue_15 (+ (.x _currentunitindex_4) 0))
  (bind _returnvalue_16 (+ (.y _currentunitindex_4) -1))
  (if (Default|IsIndexValid (Variables|Components|GetGrid) (Utilities|Struct|MakeIntPoint _returnvalue_9 _returnvalue_10))
    (Utilities|Array|AddUnique (Variables|UnitReachableTiles|GetReachableIndexes) (Utilities|Struct|MakeIntPoint _returnvalue_9 _returnvalue_10)))
  (if (Default|IsIndexValid (Variables|Components|GetGrid) (Utilities|Struct|MakeIntPoint _returnvalue_15 _returnvalue_16))
    (Utilities|Array|AddUnique (Variables|UnitReachableTiles|GetReachableIndexes) (Utilities|Struct|MakeIntPoint _returnvalue_15 _returnvalue_16)))
  (if (Default|IsIndexValid (Variables|Components|GetGrid) (Utilities|Struct|MakeIntPoint _returnvalue_3 _returnvalue_4))
    (Utilities|Array|AddUnique (Variables|UnitReachableTiles|GetReachableIndexes) (Utilities|Struct|MakeIntPoint _returnvalue_3 _returnvalue_4)))
  (if (Default|IsIndexValid (Variables|Components|GetGrid) (Utilities|Struct|MakeIntPoint _returnvalue_7 _returnvalue_8))
    (Utilities|Array|AddUnique (Variables|UnitReachableTiles|GetReachableIndexes) (Utilities|Struct|MakeIntPoint _returnvalue_7 _returnvalue_8)))
  (if (Default|IsIndexValid (Variables|Components|GetGrid) (Utilities|Struct|MakeIntPoint _returnvalue_11 _returnvalue_12))
    (Utilities|Array|AddUnique (Variables|UnitReachableTiles|GetReachableIndexes) (Utilities|Struct|MakeIntPoint _returnvalue_11 _returnvalue_12)))
  (if (Default|IsIndexValid (Variables|Components|GetGrid) (Utilities|Struct|MakeIntPoint _returnvalue_13 _returnvalue_14))
    (Utilities|Array|AddUnique (Variables|UnitReachableTiles|GetReachableIndexes) (Utilities|Struct|MakeIntPoint _returnvalue_13 _returnvalue_14)))
  (if (Default|IsIndexValid (Variables|Components|GetGrid) (Utilities|Struct|MakeIntPoint _returnvalue_5 _returnvalue_6))
    (Utilities|Array|AddUnique (Variables|UnitReachableTiles|GetReachableIndexes) (Utilities|Struct|MakeIntPoint _returnvalue_5 _returnvalue_6)))
  (if (Default|IsIndexValid (Variables|Components|GetGrid) (Utilities|Struct|MakeIntPoint _returnvalue_2 _returnvalue))
    (Utilities|Array|AddUnique (Variables|UnitReachableTiles|GetReachableIndexes) (Utilities|Struct|MakeIntPoint _returnvalue_2 _returnvalue))))

(fn ResetReachableTiles
  (for _array_element (Variables|UnitReachableTiles|GetReachableIndexes)
    (Default|RemoveStatefromTile (Variables|Components|GetGrid) _array_element "NewEnumerator3")))

(fn SetReachableTiles
  (for _array_element (Variables|UnitReachableTiles|GetReachableIndexes)
    (Default|AddStatetoTile (Variables|Components|GetGrid) _array_element "NewEnumerator3")))

(fn MoveSelectedUnit
  (params (Index :type Int%20Point%20Structure))
  (Utilities|IsValid (Variables|References|GetSelectedUnit)
    (:Is%20Valid
      (bind _index (Default|GetTileIndexUnderCursor (Variables|Components|GetGrid)))
      (LocalVariables|SetSelectedMoveTile _index)
      (if (Utilities|Array|ContainsItem (Variables|UnitReachableTiles|GetReachableIndexes) _index)
        (bind _unitontile (Actions|UnitonTile _index))
        (if (not (Utilities|IsValid _unitontile))
          (Default|MovedUnitinCombat (Variables|Components|GetCombatSystem) (Variables|References|GetSelectedUnit) _index)
          (Actions|SetSelectedTileandUnit (LocalVariables|GetSelectedMoveTile)) ; Once the unit index has been moved call the set selected function to set new index
        )))))

(fn UnitonTile
  (params (Index :type Int%20Point%20Structure))
  (return (.UnitOnTile (Utilities|Struct|BreakS_TileData (.Value (Utilities|Map|Find (Variables|/Game/Core/Grid/BP_Grid.BP_Grid_C|GetGridTiles (Variables|Components|GetGrid)) Index))))))

(fn CreateDefaultUnits
  (bind _combatsystem (Variables|Components|GetCombatSystem))
  (bind _combatsystem_2 (Variables|Components|GetCombatSystem))
  (bind _combatsystem_3 (Variables|Components|GetCombatSystem))
  (bind _returnvalue (Game|SpawnActorfromClass "/Game/Core/Units/BP_Unit.BP_Unit_C" (Math|Transform|MakeTransform "0, 0, 0" "0.000000,90.000000,0.000000" "1.000000,1.000000,1.000000") "AlwaysSpawn" "MultiplyWithRoot" 0 "NewEnumerator0" 0))
  (Default|AddUnitinCombat _combatsystem_2 _returnvalue (Utilities|Struct|MakeIntPoint 6 1))
  (bind _returnvalue_2 (Game|SpawnActorfromClass "/Game/Core/Units/BP_Unit.BP_Unit_C" (Math|Transform|MakeTransform "0, 0, 0" "0.000000,90.000000,0.000000" "1.000000,1.000000,1.000000") "AlwaysSpawn" "MultiplyWithRoot" 0 "NewEnumerator0" 0))
  (Default|AddUnitinCombat _combatsystem_2 _returnvalue_2 (Utilities|Struct|MakeIntPoint 5 1))
  (bind _returnvalue_3 (Game|SpawnActorfromClass "/Game/Core/Units/BP_Unit.BP_Unit_C" (Math|Transform|MakeTransform "0, 0, 0" "0.000000,90.000000,0.000000" "1.000000,1.000000,1.000000") "AlwaysSpawn" "MultiplyWithRoot" 0 "NewEnumerator1" 0))
  (Default|AddUnitinCombat _combatsystem_3 _returnvalue_3 (Utilities|Struct|MakeIntPoint 7 1))
  (bind _returnvalue_4 (Game|SpawnActorfromClass "/Game/Core/Units/BP_Unit.BP_Unit_C" (Math|Transform|MakeTransform "0, 0, 0" "0.000000,90.000000,0.000000" "1.000000,1.000000,1.000000") "AlwaysSpawn" "MultiplyWithRoot" 0 "NewEnumerator1" 0))
  (Default|AddUnitinCombat _combatsystem_3 _returnvalue_4 (Utilities|Struct|MakeIntPoint 4 1))
  (bind _returnvalue_5 (Game|SpawnActorfromClass "/Game/Core/Units/BP_Unit.BP_Unit_C" (Math|Transform|MakeTransform "0, 0, 0" "0.000000,90.000000,0.000000" "1.000000,1.000000,1.000000") "AlwaysSpawn" "MultiplyWithRoot" 0 "NewEnumerator2" 0))
  (Default|AddUnitinCombat _combatsystem _returnvalue_5 (Utilities|Struct|MakeIntPoint 8 0))
  (bind _returnvalue_6 (Game|SpawnActorfromClass "/Game/Core/Units/BP_Unit.BP_Unit_C" (Math|Transform|MakeTransform "0, 0, 0" "0.000000,90.000000,0.000000" "1.000000,1.000000,1.000000") "AlwaysSpawn" "MultiplyWithRoot" 0 "NewEnumerator2" 0))
  (Default|AddUnitinCombat _combatsystem _returnvalue_6 (Utilities|Struct|MakeIntPoint 3 0)))

(fn OnCombatStarted
  (Actions|SetSelectedActions)
  (Actions|SetSelectedTileandUnit (Utilities|Struct|MakeIntPoint -999 -999))
  (bind _returnvalue (UserInterface|CreateWidget "/Game/Core/Combat/Widgets/W_Combat.W_Combat_C" 0 self))
  (bind _output_get (Variables|References|SetW_Combat _returnvalue))
  (UserInterface|Viewport|AddtoPlayerScreen _output_get)
  (EventDispatchers|BindEventtoOnSelectedSpellButtonChange (Variables|/Game/Core/Combat/Widgets/W_Combat.W_Combat_C|GetButtonList_Spells (Variables|References|GetW_Combat)) (EventDispatchers|CreateEvent :!event OnSelectedSpellChange)))

(fn OnCombatEnded
  (Actions|SetSelectedActions)
  (Actions|SetSelectedTileandUnit (Utilities|Struct|MakeIntPoint -999 -999))
  (Widget|RemovefromParent (Variables|References|GetW_Combat))
  (Variables|References|SetW_Combat 0))

(fn OnUnitTurnStarted
  (params (Unit :type BP%20Unit%20Object%20Reference))
  (Actions|SetSelectedTileandUnit (Variables|/Game/Core/Units/BP_Unit.BP_Unit_C|GetIndex Unit))
  (Actions|SetSelectedActions "/Game/Core/Player/Actions/Grid/Action_MoveUnitOnGrid.Action_MoveUnitOnGrid_C")
  (Default|LinkUnittoSpellList (Variables|/Game/Core/Combat/Widgets/W_Combat.W_Combat_C|GetButtonList_Spells (Variables|References|GetW_Combat)) (Variables|References|GetSelectedUnit)))

(fn OnUnitTurnEnded
  (params (Unit :type BP%20Unit%20Object%20Reference))
  (Actions|SetSelectedTileandUnit (Utilities|Struct|MakeIntPoint -999 -999))
  (Default|LinkUnittoSpellList (Variables|/Game/Core/Combat/Widgets/W_Combat.W_Combat_C|GetButtonList_Spells (Variables|References|GetW_Combat))))

(fn OnSelectedSpellChange
  (params (Button :type Button%20Spell%20Object%20Reference))
  (Utilities|IsValid Button
    (:Is%20Valid
      (Actions|SetSelectedActions "/Game/Core/Player/Actions/Combat/Action_Combat_CastSpell.Action_Combat_CastSpell_C")
      (bind _asaction_combat_cast_spell (Utilities|Casting|CastToAction_Combat_CastSpell (Variables|Actions|GetSelectedAction_LeftClick)))
      (Default|SetSpell _asaction_combat_cast_spell (Variables|/Game/Core/Combat/Spells/Widgets/Button_Spell.Button_Spell_C|GetSpell Button)))
    (:Is%20Not%20Valid
      (if (!= (Utilities|GetClass (Variables|Actions|GetSelectedAction_LeftClick)) "/Game/Core/Player/Actions/Grid/Action_MoveUnitOnGrid.Action_MoveUnitOnGrid_C")
        (Actions|SetSelectedActions "/Game/Core/Player/Actions/Grid/Action_MoveUnitOnGrid.Action_MoveUnitOnGrid_C")))))