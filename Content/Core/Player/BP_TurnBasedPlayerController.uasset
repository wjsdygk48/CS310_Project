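; Player controller for a turn-based hero game that lets a player select, move and attack with heroes during their turn.
; A left-click traces under the cursor to select an owned hero, then target another player's hero or a location.
; Server actions issue AI moves and advance turns through the game mode without waiting for movement; attacks currently only advance the turn.
; Client turn events toggle input handling and broadcast the change.
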(event Custom|StartTurn%20CLIENT
  (CallFunction|SetMyTurn true))

(event Custom|EndTurn%20CLIENT
  (CallFunction|SetMyTurn false))

(event Custom|SetPlayerIndex
  (params (PlayerIndex :type Integer))
  (Variables|Default|SetPlayer%20Index PlayerIndex))

(event Custom|ServerAction%20-%20Attack%20Hero
  (params (AttackingHero :type BP%20Hero%20Object%20Reference) (AttackedHero :type BP%20Hero%20Object%20Reference))
  (bind _asturn_based_game_mode (Utilities|Casting|CastToTurnBasedGameMode (Game|GetGameMode)))
  (Default|CycleTurns _asturn_based_game_mode))

(event Custom|ServerAction%20-%20Move%20Hero
  (params (Hero :type BP%20Hero%20Object%20Reference) (Location :type Vector))
  (AI|Navigation|MovetoLocation (AI|GetAIController Hero) Location -1.0 true true false true 0)
  (bind _asturn_based_game_mode (Utilities|Casting|CastToTurnBasedGameMode (Game|GetGameMode)))
  (Default|CycleTurns _asturn_based_game_mode))

(event EventBeginPlay)

(event Input|MouseEvents|LeftMouseButton
  (params (Key :type Key%20Structure :default "None"))
  (:Pressed
    (if (Variables|Default|GetMyTurn?)
      (CallFunction|HandleLeftMouseButton))))

(fn ConstructionScript)

(fn SetMyTurn
  (params (MyTurn? :type Boolean))
  (bind _output_get (Variables|Default|SetMyTurn? MyTurn?))
  (Default|CallOnMyTurnChanged _output_get))

(fn HandleLeftMouseButton
  (bind (_hitresult _returnvalue) (Game|Player|GetHitResultUnderCursorbyChannel "TraceTypeQuery2" true))
  (bind (_bblockinghit _binitialoverlap _time _distance _location _impactpoint _normal _impactnormal _physmat _hitactor) (Collision|BreakHitResult _hitresult))
  (Utilities|FlowControl|Sequence
    (:then_0
      (if _returnvalue
        (LocalVariables|SetNewlySelectedLocation _impactpoint)
        (bind _asbp_hero (Utilities|Casting|CastToBP_Hero _hitactor))
        (LocalVariables|SetNewlySelectedActor _asbp_hero)
        (else
          (return))))
    (:then_1
      (if (!= (Variables|Default|GetSelectedHero) (LocalVariables|GetNewlySelectedActor))
        (bind _newlyselectedactor (LocalVariables|GetNewlySelectedActor)
          (:then
            (if (== (Default|GetPlayerIndex _newlyselectedactor) (Variables|Default|GetPlayer%20Index))
              (Variables|Default|SetSelectedHero (LocalVariables|GetNewlySelectedActor))
              (else
                (bind _selectedhero (Variables|Default|GetSelectedHero)
                  (:then
                    (CallFunction|ServerAction-AttackHero _selectedhero (LocalVariables|GetNewlySelectedActor))
                    (Variables|Default|SetSelectedHero 0))
                  (:else)))))
          (:else
            (bind _selectedhero_2 (Variables|Default|GetSelectedHero)
              (:then
                (CallFunction|ServerAction-MoveHero _selectedhero_2 (LocalVariables|GetNewlySelectedLocation))
                (Variables|Default|SetSelectedHero 0))
              (:else))))))))