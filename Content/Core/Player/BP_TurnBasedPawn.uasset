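; BP_TurnBasedPawn is the player pawn for turn-based play, acting as a free-moving camera driven by a BP_TurnBasedPlayerController.
; Axis inputs move it along its forward, right and world up vectors, scaled by CameraSpeed.
; Holding right mouse hides the cursor and turns mouse movement into yaw and inverted pitch.
; During the hold, Tick pins the cursor to the viewport center; release restores its saved position and visibility.
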(event EventTick
  (params (DeltaSeconds :type Float%20%28single-precision%29))
  (bind _returnvalue (Viewport|GetViewportSize))
  (if (Variables|Default|GetRightMouseButtonDown)
    (Class|PlayerController|SetMouseLocation (Variables|Default|GetPlayerController) (Math|Float|Truncate (/ (.x _returnvalue) 2.0)) (Math|Float|Truncate (/ (.y _returnvalue) 2.0)))))

(event EventBeginPlay
  (bind _asturn_based_player_controller (Utilities|Casting|CastToBP_TurnBasedPlayerController (Pawn|GetController)))
  (Variables|Default|SetPlayerController _asturn_based_player_controller))

(event Input|AxisEvents|InputAxisMoveX
  (params (AxisValue :type Float%20%28single-precision%29))
  (Pawn|Input|AddMovementInput (Transformation|GetActorForwardVector) (* AxisValue (Variables|Default|GetCameraSpeed)) false))

(event Input|AxisEvents|InputAxisMoveY
  (params (AxisValue :type Float%20%28single-precision%29))
  (Pawn|Input|AddMovementInput (Transformation|GetActorRightVector) (* AxisValue (Variables|Default|GetCameraSpeed)) false))

(event Input|AxisEvents|InputAxisMoveZ
  (params (AxisValue :type Float%20%28single-precision%29))
  (Pawn|Input|AddMovementInput (Math|Vector|VectorUp) (* AxisValue (Variables|Default|GetCameraSpeed)) false))

(event Input|MouseEvents|MouseX
  (params (AxisValue :type Float%20%28single-precision%29))
  (if (Variables|Default|GetRightMouseButtonDown)
    (Pawn|Input|AddControllerYawInput AxisValue)))

(event Input|MouseEvents|MouseY
  (params (AxisValue :type Float%20%28single-precision%29))
  (if (Variables|Default|GetRightMouseButtonDown)
    (Pawn|Input|AddControllerPitchInput (* AxisValue -1.0))))

(event Input|MouseEvents|RightMouseButton
  (params (Key :type Key%20Structure))
  (bind _playercontroller (Variables|Default|GetPlayerController))
  (bind (_locationx _locationy) (Game|Player|GetMousePosition _playercontroller))
  (:Pressed
    (Variables|/Script/Engine.PlayerController|SetbShowMouseCursor (Variables|Default|GetPlayerController) false)
    (Utilities|FlowControl|Delay 0.0)
    (Variables|Default|SetRightMouseButtonDown true)
    (Variables|Default|SetMouseSavedPosition (Utilities|Struct|MakeIntPoint (Math|Float|Truncate _locationx) (Math|Float|Truncate _locationy))))
  (:Released
    (Variables|Default|SetRightMouseButtonDown false)
    (Class|PlayerController|SetMouseLocation (Variables|Default|GetPlayerController) (.x (Variables|Default|GetMouseSavedPosition)) (.y (Variables|Default|GetMouseSavedPosition)))
    (Utilities|FlowControl|Delay 0.0)
    (Variables|/Script/Engine.PlayerController|SetbShowMouseCursor (Variables|Default|GetPlayerController) true)))

(fn ConstructionScript)