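; BP_SpellAnimation plays a spell's visual on the combat grid and signals when it has finished.
; On BeginPlay it spawns a capsule BP_AnimatedShape per target index, given the origin tile's location and rotation at tiny scale and the target tile's transform to animate toward.
; Only the first shape's completion event is bound, and it fires OnSpellAnimationCompleted for the whole spell.
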(event Custom|Event_PlaySpellAnimation
  (bind _originindex (Variables|Default|GetOriginIndex))
  (bind _transform (CallFunction|GetTileTransform _originindex))
  (for (_array_element _array_index) (Variables|Default|GetTargetIndexes)
    (bind _returnvalue (Game|SpawnActorfromClass "/Game/Core/Combat/Spells/Components/BP_AnimatedShape.BP_AnimatedShape_C" (Math|Transform|MakeTransform "0, 0, 0" "0, 0, 0" "1.000000,1.000000,1.000000") "AlwaysSpawn" "MultiplyWithRoot" 0 "/Game/StarterContent/Shapes/Shape_NarrowCapsule.Shape_NarrowCapsule" "/Game/StarterContent/Materials/M_Basic_Wall.M_Basic_Wall" "(R=1.000000,G=0.008681,B=0.000000,A=1.000000)" (Math|Transform|MakeTransform (.location _transform) (.rotation _transform) "0.010000,0.010000,0.010000") (CallFunction|GetTileTransform _array_element) 0))
    (if (== _array_index 0)
      (EventDispatchers|BindEventtoOnShapeAnimationCompleted _returnvalue (delegate Custom|OnShapeAnimationCompleted)))))

(event Custom|OnShapeAnimationCompleted
  (params (Animated%20Shape :type BP%20Animated%20Shape%20Object%20Reference))
  (CallFunction|EventCompleteSpellAnimation))

(event Custom|Event_CompleteSpellAnimation
  (Default|CallOnSpellAnimationCompleted self))

(event EventBeginPlay
  (CallFunction|EventPlaySpellAnimation))

(fn ConstructionScript)

(fn GetTileTransform
  (params (Index :type Int%20Point%20Structure%20%28by%20ref%29))
  (return (Utilities|Struct|BreakS_TileData (.Value (Utilities|Map|Find (Variables|/Game/Core/Grid/BP_Grid.BP_Grid_C|GetGridTiles (Variables|Default|GetGrid)) Index)))))