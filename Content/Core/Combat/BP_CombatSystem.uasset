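; BP_CombatSystem tracks units in combat on a tile grid and handles spell casting.
; Adding, moving and removing units all route through SetUnitIndexOnGrid, which updates tile occupancy and teleports the unit to its tile.
; Removal uses a sentinel index, sending the unit to a far off-grid location.
; CastSpell checks the target against the spell's pattern-based range, then spawns its animation actor with the grid, origin and single target index.
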(event EventBeginPlay)

(event Collision|EventActorBeginOverlap
  (params (OtherActor :type Actor%20Object%20Reference)))

(event EventTick
  (params (DeltaSeconds :type Float%20%28single-precision%29)))

(fn ConstructionScript)

(fn AddUnitinCombat
  (params (Unit :type BP%20Unit%20Object%20Reference) (Index :type Int%20Point%20Structure))
  (Utilities|Array|Add (Variables|Default|GetUnitsInCombat) Unit)
  (CallFunction|SetUnitIndexonGrid Unit Index))

(fn RemoveUnitfromCombat
  (params (Unit :type BP%20Unit%20Object%20Reference))
  (Utilities|Array|RemoveItem (Variables|Default|GetUnitsInCombat) Unit)
  (CallFunction|SetUnitIndexonGrid Unit (Utilities|Struct|MakeIntPoint -999 -999)))

(fn SetUnitIndexonGrid
  (params (Unit :type BP%20Unit%20Object%20Reference) (Index :type Int%20Point%20Structure))
  (Utilities|FlowControl|Sequence
    (:then_0
      (if (!= (Variables|/Game/Core/Units/BP_Unit.BP_Unit_C|GetIndex Unit) Index) ; Check is the same index
        (Utilities|FlowControl|Sequence ; 0 - Remove unti from previous tile, 1- add to new tile
          (:then_0
            (bind _output_get (LocalVariables|SetPreviousTile (.Value (Utilities|Map|Find (Variables|/Game/Core/Grid/BP_Grid.BP_Grid_C|GetGridTiles (Variables|Default|GetGrid)) (Variables|/Game/Core/Units/BP_Unit.BP_Unit_C|GetIndex Unit)))))
            (if (== (.UnitOnTile (Utilities|Struct|BreakS_TileData _output_get)) Unit)
              (bind _structout (Utilities|Struct|SetmembersinS_TileData (LocalVariables|GetPreviousTile)))
              (Utilities|Map|Add (Variables|/Game/Core/Grid/BP_Grid.BP_Grid_C|GetGridTiles (Variables|Default|GetGrid)) (Utilities|Struct|BreakS_TileData _structout) _structout)))
          (:then_1
            (Variables|/Game/Core/Units/BP_Unit.BP_Unit_C|SetIndex Unit Index)
            (if (!= Index (Utilities|Struct|MakeIntPoint -999 -999))
              (bind _structout_2 (Utilities|Struct|SetmembersinS_TileData (.Value (Utilities|Map|Find (Variables|/Game/Core/Grid/BP_Grid.BP_Grid_C|GetGridTiles (Variables|Default|GetGrid)) Index)) Unit))
              (Utilities|Map|Add (Variables|/Game/Core/Grid/BP_Grid.BP_Grid_C|GetGridTiles (Variables|Default|GetGrid)) (Utilities|Struct|BreakS_TileData _structout_2) _structout_2))))))
    (:then_1
      (Transformation|SetActorLocation Unit (select (.ReturnValue (Utilities|Map|Find (Variables|/Game/Core/Grid/BP_Grid.BP_Grid_C|GetGridTiles (Variables|Default|GetGrid)) Index)) (.location (Utilities|Struct|BreakS_TileData (.Value (Utilities|Map|Find (Variables|/Game/Core/Grid/BP_Grid.BP_Grid_C|GetGridTiles (Variables|Default|GetGrid)) Index)))) "-99999.000000,-99999.000000,-99999.000000") false false))))

(fn MovedUnitinCombat
  (params (Unit :type BP%20Unit%20Object%20Reference) (Index :type Int%20Point%20Structure))
  (CallFunction|SetUnitIndexonGrid Unit Index))

(fn CastSpell
  (params (Spell :type E_Spell%20Enum :default "NewEnumerator0") (Origin%20Index :type Int%20Point%20Structure) (Target%20index :type Int%20Point%20Structure))
  (bind _spell_data (CallFunction|GetSpellDatafromSpell Spell))
  (LocalVariables|SetData _spell_data)
  (bind _range_indexes (CallFunction|GetSpellRange Origin%20Index (Utilities|Struct|BreakS_SpellData (LocalVariables|GetData))))
  (if (Utilities|Array|ContainsItem _range_indexes Target%20index)
    (Game|SpawnActorfromClass (Utilities|Struct|BreakS_SpellData_Assets (.assets (LocalVariables|GetData))) (Math|Transform|MakeTransform "0, 0, 0" "0, 0, 0" "1.000000,1.000000,1.000000") "AlwaysSpawn" "MultiplyWithRoot" 0 (Variables|Default|GetGrid) Origin%20Index (Utilities|Array|MakeArray Target%20index) 0)))

(fn GetSpellRange
  (params (OriginIndex :type Int%20Point%20Structure) (Cast :type S%20Spell%20Data%20Cast%20Structure))
  (bind (_rangepattern _rangeminmax) (Utilities|Struct|BreakS_SpellData_Cast Cast))
  (bind _rangeindexes (CallFunction|GetIndexesfromPatternandRange OriginIndex _rangepattern _rangeminmax))
  (return _rangeindexes))