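; AI agent unit Blueprint that registers itself with Learning Agents and exposes an adjustable difficulty scale.
; On BeginPlay it finds the LearningAgentsManager in the level, adds itself and stores the returned AgentId, printing an error if no manager exists.
; SetDifficultyScale clamps its input between -1 and 1, prints it and broadcasts it through OnDifficultyScaleUpdated.
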(event EventBeginPlay
  (|CallParentFunction)
  (bind _returnvalue (Actor|GetActorOfClass "/Script/LearningAgents.LearningAgentsManager"))
  (Utilities|IsValid _returnvalue
    (:Is%20Valid
      (bind _returnvalue_2 (Class|LearningAgentsManager|AddAgent _returnvalue self))
      (Variables|Default|SetAgentId _returnvalue_2))
    (:Is%20Not%20Valid
      (Development|PrintString "Could not find LA manager"))))

(fn ConstructionScript)

(fn SetDifficultyScale
  (params (DifficultyScale :type Float%20%28double-precision%29))
  (bind _output_get (Variables|Default|SetDifficultyScale (Math|Float|Clamp(Float) DifficultyScale -1.0)))
  (Development|PrintString (Utilities|String|ToString(Float) _output_get))
  (Default|CallOnDifficultyScaleUpdated _output_get))