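; Ranger unit AI that varies its movement logic from turn to turn during combat by overriding its parent's AI hooks.
; A turn counter resets when combat starts and increments before each AI turn, which also clears a damage flag.
; Casting a spell sets that flag from whether its minimum HP modifier is negative.
; Movement logic selects one mode on even turns without a damaging cast, and another otherwise.
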(event EventBeginPlay
  (|CallParentFunction) ; This node is disabled and will not be called.\nDrag off pins to build functionality.
)

(event Collision|EventActorBeginOverlap
  (params (OtherActor :type Actor%20Object%20Reference)))

(event EventTick
  (params (DeltaSeconds :type Float%20%28single-precision%29)))

(event EventCastSpell
  (params (MovedBeforeCast :type Boolean))
  (bind _spell_data (CallFunction|GetSpellDatafromSpell (Utilities|Struct|BreakS_UnitAiSpellCastingData (Variables|Default|GetAiSpellCasting))))
  (Variables|Default|SetDamagedAnUnitThisTurn (< (.X (Utilities|Struct|BreakIntPoint (Utilities|Struct|BreakS_SpellData_Impact (Utilities|Struct|BreakS_SpellData _spell_data)))) 0))
  (|CallParentFunction true))

(fn ConstructionScript
  (|CallParentFunction))

(fn AiPlayTurn
  (Math|Integer|IncrementInt (Variables|Default|GetTurnCount)
    (:%20%20
      (Variables|Default|SetDamagedAnUnitThisTurn false)
      (|CallParentFunction))))

(fn GetUnitMovementLogic
  (return (select (and (CallFunction|IsIntEven (Variables|Default|GetTurnCount)) (not (Variables|Default|GetDamagedAnUnitThisTurn))) "NewEnumerator0" "NewEnumerator1")))

(fn AiCombatStarted
  (Variables|Default|SetTurnCount 0)
  (|CallParentFunction))