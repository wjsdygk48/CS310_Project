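; BP_Team1Ai is the Team 1 AI unit, which registers itself as an agent for Learning Agents.
; On BeginPlay it runs the parent logic, adds itself to the level's LearningAgentsManager and stores the returned AgentId, printing an error if no manager exists.
; SetTeam1DifficultyScale clamps and stores the difficulty scale, prints it and broadcasts it through the OnTeam1DifficultyScaleUpdated dispatcher.
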(event EventBeginPlay
  (|CallParentFunction)
  (bind _returnvalue (Actor|GetActorOfClass "/Script/LearningAgents.LearningAgentsManager"))
  (Utilities|IsValid _returnvalue
    (:Is%20Valid
      (bind _returnvalue_2 (Class|LearningAgentsManager|AddAgent _returnvalue self))
      (Variables|Default|SetAgentId _returnvalue_2))
    (:Is%20Not%20Valid
      (Development|PrintString "Could not find LA manager"))))

(event Collision|EventActorBeginOverlap
  (params (OtherActor :type Actor%20Object%20Reference)))

(event EventTick
  (params (DeltaSeconds :type Float%20%28single-precision%29)))

(fn ConstructionScript)

(fn SetTeam1DifficultyScale
  (params (DifficultyScale :type Float%20%28double-precision%29))
  (bind _output_get (Variables|Default|SetDifficultyScale (Math|Float|Clamp(Float) DifficultyScale -1.0)))
  (Development|PrintString (Utilities|String|ToString(Float) _output_get))
  (Default|CallOnTeam1DifficultyScaleUpdated _output_get))