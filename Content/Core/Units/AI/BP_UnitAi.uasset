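; AI brain for a unit in turn-based grid combat that plays its turn through delayed states: decide, move, cast, end turn.
; It brute-forces castable spells, reachable origins and targets, scoring HP impact, kill chance and travel distance, with allies weighed inversely.
; Without a move-then-cast, it repositions by the unit's movement logic, treating team 0 as enemies.
; It registers with a Learning Agents manager, though decisions are hand-scripted.
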(event Custom|OnUnitActiveInCombatChanged
  (params (Unit :type BP%20Unit%20Object%20Reference))
  (if (not (Variables|/Game/Core/Units/BP_Unit.BP_Unit_C|GetIsActiveInCombat Unit))
    (if (Utilities|Enum|NotEqual(Enum) (Variables|Default|GetAiState) "NewEnumerator6")
      (Utilities|SetAiStatewithDelay "NewEnumerator6")
      (Default|CallOnAiStateChanged self))))

(event EventBeginPlay
  (|CallParentFunction)
  (bind _returnvalue (Actor|GetActorOfClass "/Script/LearningAgents.LearningAgentsManager"))
  (Utilities|IsValid _returnvalue
    (:Is%20Valid
      (bind _returnvalue_2 (Class|LearningAgentsManager|AddAgent _returnvalue self))
      (Variables|Default|SetAgentId _returnvalue_2)
      (EventDispatchers|UnbindEventfromOnUnitActiveinCombatChanged (Variables|Default|GetUnit) (delegate Custom|OnUnitActiveInCombatChanged)))
    (:Is%20Not%20Valid
      (Development|PrintString "Could not find LA manager"))))

(event Custom|Event_RunAiLogic
  (Utilities|SetAiStatewithDelay "NewEnumerator1")
  (Utilities|SetAiStatewithDelay "NewEnumerator2")
  (CallFunction|DecideSpelltoCast))

(event Custom|TurnDone
  (Utilities|SetAiStatewithDelay "NewEnumerator6")
  (Flow|AiEndTurn))

(event Custom|DecideSpellToCast_Done
  (Utilities|SetAiStatewithDelay "NewEnumerator3")
  (CallFunction|MovetoCastLocation (Utilities|Struct|BreakS_UnitAiSpellCastingData (Variables|Default|GetAiSpellCasting))))

(event Custom|MoveToCastLocation_Done
  (Utilities|SetAiStatewithDelay "NewEnumerator4")
  (CallFunction|CastSpell true))

(event Custom|MoveToLocationAfterCast
  (bind _reachableindexes (Default|GetUnitReachableRange (Variables|Default|GetPlayerActions) (Variables|Default|GetUnit)))
  (bind _targetindex (Movement|FindBestIndexinReachables _reachableindexes))
  (Default|MoveSelectedUnitAi (Variables|Default|GetPlayerActions) _targetindex (Variables|Default|GetUnit))
  (CallFunction|TurnDone))

(event Custom|MoveToCastLocation
  (params (IsSpellValid :type Boolean))
  (bind _aispellcasting (Variables|Default|GetAiSpellCasting))
  (bind (_isspellvalid _originindex) (Utilities|Struct|BreakS_UnitAiSpellCastingData _aispellcasting))
  (if IsSpellValid
    (if (and (!= (Variables|/Game/Core/Units/BP_Unit.BP_Unit_C|GetIndex (Variables|Default|GetUnit)) _originindex) _isspellvalid)
      (Default|MoveSelectedUnitAi (Variables|Default|GetPlayerActions) (Utilities|Struct|BreakS_UnitAiSpellCastingData (Variables|Default|GetAiSpellCasting)) (Variables|Default|GetUnit))
      (CallFunction|MovetoCastLocationDone)
      (else
        (CallFunction|CastSpell (Class|KismetSystemLibrary|MakeLiteralBool false))
        (Utilities|FlowControl|Delay 0.75)
        (Utilities|StopFlowifUnitIsInactive)
        (CallFunction|MovetoLocationAfterCast)))
    (else
      (bind _reachableindexes (Default|GetUnitReachableRange (Variables|Default|GetPlayerActions) (Variables|Default|GetUnit)))
      (bind _targetindex (Movement|FindBestIndexinReachables _reachableindexes))
      (Default|MoveSelectedUnitAi (Variables|Default|GetPlayerActions) _targetindex (Variables|Default|GetUnit))
      (CallFunction|TurnDone))))

(event Custom|DecideSpellToCast
  (Variables|Default|SetAiSpellCasting "")
  (bind _reachableindexes (Default|GetUnitReachableRange (Variables|Default|GetPlayerActions) (Variables|Default|GetUnit)))
  (bind _spells (Spell|GetCastableSpells))
  (for _array_element _spells
    (for _array_element_2 _reachableindexes
      (bind _range_indexes (Default|GetSpellRange (Variables|Default|GetCombatSystem) _array_element_2 (Utilities|Struct|BreakS_SpellData _array_element)))
      (for _array_element_3 _range_indexes
        (Spell|CalculateSpellScoreandUpdateSpellCasting _array_element_3 _array_element_2 _array_element)))
    (CallFunction|DecideSpelltoCastDone)))

(event Custom|CastSpell
  (params (MovedBeforeCast :type Boolean))
  (bind _aispellcasting (Variables|Default|GetAiSpellCasting))
  (bind (_spell _originindex _targetindex) (Utilities|Struct|BreakS_UnitAiSpellCastingData _aispellcasting))
  (if (Utilities|Struct|BreakS_UnitAiSpellCastingData (Variables|Default|GetAiSpellCasting))
    (Default|CastSpell (Variables|Default|GetCombatSystem) _spell _originindex _targetindex)
    (Utilities|FlowControl|Delay 0.75)
    (Utilities|StopFlowifUnitIsInactive)
    (if MovedBeforeCast
      (CallFunction|TurnDone)
      (else
        (CallFunction|MovetoLocationAfterCast)))
    (else
      (CallFunction|TurnDone))))

(fn ConstructionScript
  (bind _returnvalue (Actor|GetActorOfClass "/Game/Core/Player/BP_PlayerActions.BP_PlayerActions_C"))
  (Variables|Default|SetPlayerActions _returnvalue))

(fn AiPlayTurn
  (CallFunction|EventRunAiLogic))

(fn AiEndTurn
  (Default|NextUnit (Variables|Default|GetCombatSystem)))

(fn FindBestIndexinReachables
  (params (Reachables :type Array%20of%20Int%20Point%20Structures))
  (bind _movementlogic (CallFunction|GetUnitMovementLogic))
  (Utilities|FlowControl|Sequence
    (:then_0
      (switch Utilities|FlowControl|Switch|SwitchonE_UnitAiMovementLogic _movementlogic
        (:NewEnumerator0
          (bind _ret (Units|GetEnemyUnits :!label _label))
          (bind _keys (Utilities|Map|Keys _ret))
          (LocalVariables|SetEnemiesOrAllies _keys))
        (:NewEnumerator3
          (bind _units (Units|GetAllyUnits false :!label _label_2))
          (bind _keys_2 (Utilities|Map|Keys _units))
          (bind _output_get (LocalVariables|SetEnemiesOrAllies _keys_2))
          (if (== (Utilities|Array|Length _output_get) 0)
            (goto _label)))
        (:NewEnumerator1
          (goto _label))
        (:NewEnumerator2
          (goto _label_2))))
    (:then_1
      (switch Utilities|FlowControl|Switch|SwitchonE_UnitAiMovementLogic _movementlogic
        (:NewEnumerator0
          _)
        (:NewEnumerator3
          _)
        (:NewEnumerator1
          (bind _index (Movement|FindFarthestIndex Reachables (LocalVariables|GetEnemiesOrAllies) :!label _label_3))
          (return _index))
        (:NewEnumerator2
          (goto _label_3)))
      (bind _index_2 (Movement|FindClosestIndex Reachables (LocalVariables|GetEnemiesOrAllies)))
      (return _index_2))))

(fn GetAllyUnits
  (params (IncludeSelf :type Boolean))
  (bind _result (Utilities|Set|ToArray (Utilities|Struct|BreakS_UnitSet (.Value (Utilities|Map|Find (Variables|/Game/Core/Combat/BP_CombatSystem.BP_CombatSystem_C|GetUnitTeams (Variables|Default|GetCombatSystem)) (Variables|/Game/Core/Units/BP_Unit.BP_Unit_C|GetTeamIndex (Variables|Default|GetUnit)))))))
  (for _array_element _result
    (LocalVariables|SetU _array_element)
    (if (Default|IsAlive (LocalVariables|GetU))
      (if (or (!= (Variables|Default|GetUnit) (LocalVariables|GetU)) IncludeSelf)
        (Utilities|Map|Add (LocalVariables|GetRet) (Variables|/Game/Core/Units/BP_Unit.BP_Unit_C|GetIndex (LocalVariables|GetU)) (LocalVariables|GetU)))))
  (return (LocalVariables|GetRet)))

(fn GetEnemyUnits
  (params (SpecificTeamIndex :type Integer))
  (bind _result (Utilities|Set|ToArray (Utilities|Struct|BreakS_UnitSet (.Value (Utilities|Map|Find (Variables|/Game/Core/Combat/BP_CombatSystem.BP_CombatSystem_C|GetUnitTeams (Variables|Default|GetCombatSystem)) SpecificTeamIndex)))))
  (for _array_element _result
    (LocalVariables|SetU _array_element)
    (if (Default|IsAlive (LocalVariables|GetU))
      (Utilities|Map|Add (LocalVariables|GetRet%20) (Variables|/Game/Core/Units/BP_Unit.BP_Unit_C|GetIndex (LocalVariables|GetU)) (LocalVariables|GetU))))
  (return (LocalVariables|GetRet%20)))

(fn FindClosestIndex
  (params (Reachables :type Array%20of%20Int%20Point%20Structures) (PossibleTargets :type Array%20of%20Int%20Point%20Structures))
  (LocalVariables|SetSmallestDistance 99999999)
  (for _array_element Reachables
    (LocalVariables|SetReachable _array_element)
    (for _array_element_2 PossibleTargets
      (LocalVariables|SetTarget _array_element_2)
      (LocalVariables|SetNewDistance (Math|Float|Truncate (Math|Vector|Distance2D(Vector) (Math|Conversions|ToVector2D(IntPoint) (LocalVariables|GetReachable)) (Math|Conversions|ToVector2D(IntPoint) (LocalVariables|GetTarget)))))
      (if (< (LocalVariables|GetNewDistance) (LocalVariables|GetSmallestDistance))
        (LocalVariables|SetRet%20%20 (LocalVariables|GetReachable))
        (LocalVariables|SetSmallestDistance (LocalVariables|GetNewDistance)))))
  (return (LocalVariables|GetRet%20%20)))

(fn FindFarthestIndex
  (params (Reachables :type Array%20of%20Int%20Point%20Structures) (IndexesToAvoid :type Array%20of%20Int%20Point%20Structures))
  (LocalVariables|SetBiggestDistance -9999999)
  (for _array_element Reachables
    (LocalVariables|SetReachable%20 _array_element)
    (LocalVariables|SetNewDistance 99999999)
    (for _array_element_2 IndexesToAvoid
      (LocalVariables|SetToAvoid _array_element_2)
      (LocalVariables|SetNewDistance (Math|Integer|Min(Integer) (LocalVariables|GetNewDistance) (Math|Float|Truncate (Math|Vector|Distance2D(Vector) (Math|Conversions|ToVector2D(IntPoint) (LocalVariables|GetReachable%20)) (Math|Conversions|ToVector2D(IntPoint) (LocalVariables|GetToAvoid)))))))
    (if (> (LocalVariables|GetNewDistance) (LocalVariables|GetBiggestDistance))
      (LocalVariables|SetRet%20%20%20 (LocalVariables|GetReachable%20))
      (LocalVariables|SetBiggestDistance (LocalVariables|GetNewDistance))))
  (return (LocalVariables|GetRet%20%20%20)))

(fn GetCastableSpells
  (for _array_element (Utilities|Struct|BreakS_UnitData_Stats (Utilities|Struct|BreakS_UnitData (Variables|/Game/Core/Units/BP_Unit.BP_Unit_C|GetUnitData (Variables|Default|GetUnit))))
    (bind _spell_data (CallFunction|GetSpellDatafromSpell _array_element))
    (bind _cancast (Default|CanCastSpell (Variables|Default|GetUnit) _spell_data))
    (if _cancast
      (Utilities|Array|Add (LocalVariables|GetRet) _spell_data)))
  (return (LocalVariables|GetRet)))

(fn CalculateSpellScoreandUpdateSpellCasting
  (params (Target :type Int%20Point%20Structure) (Origin :type Int%20Point%20Structure) (Spell :type S%20Spell%20Data%20Structure))
  (bind _allunits (Units|GetAllUnits false))
  (LocalVariables|SetAllUnitsExceptSelf _allunits)
  (bind _attackedindexes (Default|GetAttackedIndexes (Variables|Default|GetCombatSystem) Spell Target))
  (LocalVariables|SetAttackedIndexes _attackedindexes)
  (LocalVariables|SetTotalSpellScore (* (Math|Vector|Distance2D(Vector) (Math|Conversions|ToVector2D(IntPoint) (Variables|/Game/Core/Units/BP_Unit.BP_Unit_C|GetIndex (Variables|Default|GetUnit))) (Math|Conversions|ToVector2D(IntPoint) Origin)) -0.5))
  (for _array_element (LocalVariables|GetAttackedIndexes)
    (LocalVariables|SetAttackedIndex _array_element)
    (if (Class|KismetMathLibrary|EqualIntPointIntPoint (LocalVariables|GetAttackedIndex) Origin)
      (LocalVariables|SetAttackedUnit (Variables|Default|GetUnit))
      (else
        (LocalVariables|SetAttackedUnit (.Value (Utilities|Map|Find (LocalVariables|GetAllUnitsExceptSelf) (LocalVariables|GetAttackedIndex))))))
    (Utilities|IsValid (LocalVariables|GetAttackedUnit)
      (:Is%20Valid
        (bind _impactscore (Spell|CalculateImpactScore Spell (LocalVariables|GetAttackedUnit)))
        (LocalVariables|SetTotalSpellScore (+ _impactscore (LocalVariables|GetTotalSpellScore))))))
  (if (> (LocalVariables|GetTotalSpellScore) (Utilities|Struct|BreakS_UnitAiSpellCastingData (Variables|Default|GetAiSpellCasting)))
    (Variables|Default|SetAiSpellCasting (Utilities|Struct|MakeS_UnitAiSpellCastingData true (Utilities|Struct|BreakS_SpellData Spell) Origin Target (LocalVariables|GetTotalSpellScore)))))

(fn GetAllUnits
  (params (IncludeSelf :type Boolean))
  (for _array_element (Variables|/Game/Core/Combat/BP_CombatSystem.BP_CombatSystem_C|GetUnitsInCombat (Variables|Default|GetCombatSystem))
    (LocalVariables|SetU _array_element)
    (if (Default|IsAlive (LocalVariables|GetU))
      (if (or (!= (LocalVariables|GetU) (Variables|Default|GetUnit)) IncludeSelf)
        (Utilities|Map|Add (LocalVariables|GetRet) (Variables|/Game/Core/Units/BP_Unit.BP_Unit_C|GetIndex (LocalVariables|GetU)) (LocalVariables|GetU)))))
  (return (LocalVariables|GetRet)))

(fn CalculateImpactScore
  (params (Spell :type S%20Spell%20Data%20Structure) (AttackedUnit :type BP%20Unit%20Object%20Reference))
  (bind _impact (Utilities|Struct|BreakS_SpellData Spell))
  (bind _impact_2 (Utilities|Struct|BreakS_SpellData Spell))
  (bind _minmaxmodifier_hp (Utilities|Struct|BreakS_SpellData_Impact _impact))
  (bind _minmaxmodifier_hp_2 (Utilities|Struct|BreakS_SpellData_Impact _impact_2))
  (bind (_x _y) (Utilities|Struct|BreakIntPoint _minmaxmodifier_hp))
  (bind (_x_2 _y_2) (Utilities|Struct|BreakIntPoint _minmaxmodifier_hp_2))
  (bind _returnvalue (Math|Integer|Absolute(Integer) _x_2))
  (bind _returnvalue_2 (+ _x _y))
  (bind _returnvalue_3 (Math|Conversions|ToFloat(Integer) _returnvalue))
  (bind _returnvalue_4 (/ _returnvalue_2 2))
  (LocalVariables|SetApValue 5.0)
  (LocalVariables|SetKillingBlowValue 1e+02)
  (Utilities|FlowControl|Sequence
    (:then_0
      (LocalVariables|SetCost (+ (LocalVariables|GetApValue) 0.0))
      (LocalVariables|SetIsAlly (== (Variables|/Game/Core/Units/BP_Unit.BP_Unit_C|GetTeamIndex (Variables|Default|GetUnit)) (Variables|/Game/Core/Units/BP_Unit.BP_Unit_C|GetTeamIndex AttackedUnit)))
      (LocalVariables|SetHpScore (Math|Conversions|ToFloat(Integer) (* (Math|Integer|Absolute(Integer) _returnvalue_4) (select (== (> _returnvalue_4 0) (LocalVariables|GetIsAlly)) 1 -1))))
      (LocalVariables|SetKillingBlowScore (* (LocalVariables|GetKillingBlowValue) (Math|Float|Clamp(Float) (- 1.0 (/ (- (Math|Conversions|ToFloat(Integer) (Utilities|Struct|BreakS_UnitData_Stats (Utilities|Struct|BreakS_UnitData (Variables|/Game/Core/Units/BP_Unit.BP_Unit_C|GetUnitData AttackedUnit)))) _returnvalue_3) (- (+ (Math|Conversions|ToFloat(Integer) (Math|Integer|Absolute(Integer) _y_2)) 1.0) _returnvalue_3)))) (select (LocalVariables|GetIsAlly) -1.0 1.0))))
    (:then_1
      (return (/ (+ (LocalVariables|GetHpScore) (LocalVariables|GetKillingBlowScore)) (Math|Float|Max(Float) (LocalVariables|GetCost) 1.0))))))

(fn GetUnitMovementLogic
  (return (.MovementLogic (Utilities|Struct|BreakS_UnitData_Ai (Utilities|Struct|BreakS_UnitData (Variables|/Game/Core/Units/BP_Unit.BP_Unit_C|GetUnitData (Variables|Default|GetUnit)))))))

(fn AiCombatStarted)

(fn AiCombatEnded)