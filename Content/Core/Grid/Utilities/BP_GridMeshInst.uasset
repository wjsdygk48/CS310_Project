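; Grid utility actor that draws tiles as instances of one InstancedStaticMesh, with its mesh, material, colour and collision set through InitialiseGridMeshInst.
; AddInstance replaces any existing instance for a tile index, using a parallel InstanceIndexes array to map tile indices to instance indices.
; Each tile's states resolve to one colour by priority (spell AOE, spell range, selected, hovered, reachable), written as RGB into per-instance custom data.
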(event EventBeginPlay
  (Actor|Tick|SetActorTickEnabled false))

(event Collision|EventActorBeginOverlap
  (params (OtherActor :type Actor%20Object%20Reference)))

(event EventTick
  (params (DeltaSeconds :type Float%20%28single-precision%29)))

(fn ConstructionScript)

(fn AddInstance
  (params (Index :type Int%20Point%20Structure%20%28by%20ref%29) (Transform :type Transform%20%28by%20ref%29) (State :type Array%20of%20E_TileState%20Enums :default "NewEnumerator0"))
  (bind _instancedstaticmesh (Variables|Default|GetInstancedStaticMesh))
  (CallFunction|RemoveInstance Index)
  (Components|InstancedStaticMesh|AddInstance (Variables|Default|GetInstancedStaticMesh) Transform false)
  (bind _returnvalue (Utilities|Array|Add (Variables|Default|GetInstanceIndexes) Index))
  (LocalVariables|SetI _returnvalue)
  (bind _colour (CallFunction|GetColourfromStates State))
  (Components|InstancedStaticMesh|SetCustomDataValue _instancedstaticmesh (LocalVariables|GetI) 0 (.R (Math|Color|BreakColor _colour)) false)
  (Components|InstancedStaticMesh|SetCustomDataValue _instancedstaticmesh (LocalVariables|GetI) 1 (.G (Math|Color|BreakColor _colour)) false)
  (Components|InstancedStaticMesh|SetCustomDataValue _instancedstaticmesh (LocalVariables|GetI) 2 (.B (Math|Color|BreakColor _colour)) false))

(fn RemoveInstance
  (params (Index :type Int%20Point%20Structure%20%28by%20ref%29))
  (bind _instanceindexes (Variables|Default|GetInstanceIndexes))
  (if (Utilities|Array|ContainsItem :TargetArray _instanceindexes)
    (Class|InstancedStaticMeshComponent|RemoveInstance (Variables|Default|GetInstancedStaticMesh) (Utilities|Array|FindItem _instanceindexes Index))
    (Utilities|Array|RemoveItem (Variables|Default|GetInstanceIndexes) Index)))

(fn ClearInstances
  (Components|InstancedStaticMesh|ClearInstances (Variables|Default|GetInstancedStaticMesh))
  (Utilities|Array|Clear (Variables|Default|GetInstanceIndexes)))

(fn InitialiseGridMeshInst
  (params (Mesh :type Static%20Mesh%20Object%20Reference) (Material :type Material%20Interface%20Object%20Reference) (Colour :type Linear%20Color%20Structure) (Collision :type ECollisionEnabled%20Enum :default "NoCollision"))
  (bind _instancedstaticmesh (Variables|Default|GetInstancedStaticMesh))
  (Components|StaticMesh|SetStaticMesh _instancedstaticmesh Mesh)
  (Rendering|Material|SetMaterial _instancedstaticmesh 0 Material)
  (Rendering|Material|SetVectorParameterValueonMaterials _instancedstaticmesh "None" (Math|Conversions|ToVector(LinearColor) Colour))
  (Collision|SetCollisionEnabled _instancedstaticmesh Collision))

(fn GetColourfromStates
  (params (States :type Array%20of%20E_TileState%20Enums :default "NewEnumerator0"))
  (if (== (Utilities|Array|Length States) 0)
    (return "(R=1.000000,G=1.000000,B=1.000000,A=1.000000)")
    (else
      (for _array_element (Utilities|Array|MakeArray "NewEnumerator5" "NewEnumerator4" "NewEnumerator2" "NewEnumerator1" "NewEnumerator3")
        (if (Utilities|Array|ContainsItem States _array_element)
          (return (Utilities|Select :Index _array_element :NewEnumerator0 "(R=1.000000,G=1.000000,B=1.000000,A=1.000000)" :NewEnumerator1 "(R=1.000000,G=0.795573,B=0.182292,A=1.000000)" :NewEnumerator2 "(R=0.125490,G=1.000000,B=0.156863,A=1.000000)" :NewEnumerator3 "(R=0.125490,G=0.811765,B=0.890196,A=1.000000)" :NewEnumerator4 "(R=0.869792,G=0.223518,B=0.090603,A=1.000000)" :NewEnumerator5 "(R=1.000000,G=0.049340,B=0.009540,A=1.000000)"))))
      (return "(R=1.000000,G=1.000000,B=1.000000,A=1.000000)"))))